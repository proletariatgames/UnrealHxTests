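; Blueprint class that exercises calls from Blueprint functions into Haxe functions, passing values and structs across and back.
; RunBlueprints forwards its string with a fixed integer to RunHaxeFunction and returns the result.
; RunBlueprints2 passes an array of POD structs to RunHaxeFunction2, then derives its outputs from the results by tagging strings and subtracting integers, so the Blueprint's processing shows in what it returns.
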(fn `runBlueprints`
  (params (str :type String))
  (returns (ReturnValue :type Integer))
  (bind _returnvalue (`self.runHaxeFunction` 42 str))
  (return _returnvalue))

(fn `runBlueprints2`
  (returns (str :type Text) (i :type Integer) (ReturnValue :type String))
  (bind (_str _i _returnvalue) (`self.runHaxeFunction2` (`|MakeArray` (make `PODStruct` 42) (make `PODStruct` 44) (make `PODStruct` 4242))))
  (bind _returnvalue_2 (`KismetStringLibrary.Concat_StrStr` "BP " (`KismetTextLibrary.Conv_TextToString` _str)))
  (return (`KismetTextLibrary.Conv_StringToText` _returnvalue_2) (- _i _returnvalue) (`KismetStringLibrary.Concat_StrStr` _returnvalue_2 " returned")))